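; BP_Score is an actor Blueprint that tracks the player's score and checks it against the saved best score.
; IncreaseScore adds one to Score.
; ComparisonScore loads or creates the saved score, calls RenuwalBestScore unless that value is higher, and returns the current score with a renewal flag.
; A tie with the saved score also counts as a new best.
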(fn ConstructionScript)

(fn IncreaseScore
  (Math|Integer|IncrementInt (Variables|Default|GetScore)))

(fn ComparisonScore
  (bind _score (Variables|Default|GetScore))
  (bind _returnvalue (Class|Score|LoadorCreateSaveGameScore))
  (if (> _returnvalue (Variables|Default|GetScore))
    (return false (Variables|Default|GetScore))
    (else
      (Class|Score|RenuwalBestScore _score)
      (return true _score))))